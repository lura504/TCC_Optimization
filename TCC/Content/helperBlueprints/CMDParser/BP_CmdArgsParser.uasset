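; BP_CmdArgsParser is a helper Blueprint that reads the game's command line to set an enum, apparently a camera selection.
; On Init it searches for the first switch string in CmdSwitches and takes the single character that follows it.
; StringToEnum converts that character to an integer and maps 0 to 3 onto the Enum variable, so only single-digit values are supported.
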(event `self.ReceiveInit`
  (bind _cmdswitches_switchcommands (break `/Game/helperBlueprints/CMDParser/STRUCT_CmdSwitches` (`self.cmdSwitches`)))
  (bind _output (`|GetArrayItem` _cmdswitches_switchcommands))
  (bind _returnvalue (`KismetSystemLibrary.GetCommandLine`))
  (bind _returnvalue_2 (`KismetStringLibrary.FindSubstring` _returnvalue _output true))
  (if (> _returnvalue_2 -1)
    (`self.String to Enum` (`KismetStringLibrary.GetSubstring` _returnvalue (+ _returnvalue_2 (`KismetStringLibrary.Len` _output))))))

(fn `String to Enum`
  (params (Camera :type "String (by ref)"))
  (switch `int` (`KismetStringLibrary.Conv_StringToInt` Camera)
    (:`0`
      (set `self.enum` "NewEnumerator0"))
    (:`1`
      (set `self.enum` "NewEnumerator1"))
    (:`2`
      (set `self.enum` "NewEnumerator2"))
    (:`3`
      (set `self.enum` "NewEnumerator3")))
  (return))